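; Game instance that tracks data-driven progression, turning reported gameplay events into door, spawn and completion actions.
; ReportEvent keys a counter map by condition type and target, currently storing zero and ignoring Amount, then evaluates every DT_ProgressionSteps row.
; Enemy and item steps compare counters to required amounts, while location and flag steps only need the key.
; Door and spawn actions fire dispatchers; only Set Flag marks steps completed.
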(event `/Game/ThirdPerson/Progression/BPI_Progression.ReportEventRemote`
  (params (ConditionType :type "/Game/ThirdPerson/Progression/E_ConditionType Enum" :default "NewEnumerator0") (ConditionTarget :type Name) (Amount :type Integer))
  (`self.ReportEvent` ConditionType ConditionTarget Amount))

(fn `EvaluateSteps`
  (bind _outrownames (`DataTableFunctionLibrary.GetDataTableRowNames` "/Game/ThirdPerson/Progression/DT_ProgressionSteps.DT_ProgressionSteps"))
  (for _array_element _outrownames
    (bind _returnvalue (`|GetDataTableRow` "/Game/ThirdPerson/Progression/DT_ProgressionSteps.DT_ProgressionSteps" _array_element)
      (:`then`
        (bind (_stepid _conditiontype _conditiontarget _requiredamount) (break `/Game/ThirdPerson/Progression/S_ProgressionStep` _returnvalue))
        (if (not (`BlueprintSetLibrary.Set_Contains` (`self.CompletedSteps`) _stepid))
          (switch `/Game/ThirdPerson/Progression/E_ConditionType` _conditiontype
            (:`NewEnumerator0`
              (bind _returnvalue_2 (`KismetStringLibrary.Conv_StringToName` (`KismetStringLibrary.Concat_StrStr` (`|GetEnumeratorNameAsString` _conditiontype) ":" (`KismetStringLibrary.Conv_NameToString` _conditiontarget))))
              (bind _value (`self.GetCounter` _returnvalue_2))
              (if (>= _value _requiredamount)
                (`self.ExecuteAction` _returnvalue :!label _label)))
            (:`NewEnumerator1`
              (bind _value_2 (`self.GetFlag` _returnvalue_2))
              (if _value_2
                (goto _label)))
            (:`NewEnumerator2`
              (bind _value_3 (`self.GetCounter` _returnvalue_2))
              (if (>= _value_3 _requiredamount)
                (goto _label)))
            (:`NewEnumerator3`
              (bind _value_4 (`self.GetFlag` _returnvalue_2))
              (if _value_4
                (goto _label)))))))))

(fn `ExecuteAction`
  (params (Row :type "/Game/ThirdPerson/Progression/S_ProgressionStep Structure"))
  (bind (_stepid _conditiontype _conditiontarget _requiredamount _actiontype _actiontarget) (break `/Game/ThirdPerson/Progression/S_ProgressionStep` Row))
  (switch `/Game/ThirdPerson/Progression/E_ActionType` _actiontype
    (:`NewEnumerator0`
      (`self.OnOpenDoor` _actiontarget))
    (:`NewEnumerator1`
      (`self.OnSpawnActor` _actiontarget))
    (:`NewEnumerator2`
      (`BlueprintSetLibrary.Set_Add` (`self.CompletedSteps`) _stepid))))

(fn `GetCounter`
  (params (Key :type Name))
  (returns (Value :type Integer))
  (bind (_value _returnvalue) (`BlueprintMapLibrary.Map_Find` (`self.ProgressionCounters`) Key))
  (if _returnvalue
    (return _value)
    (else
      (return 0))))

(fn `GetFlag`
  (params (Key :type Name))
  (returns (Value :type Boolean))
  (return (`.ReturnValue` (`BlueprintMapLibrary.Map_Find` (`self.ProgressionCounters`) Key))))

(fn `ReportEvent`
  (params (ConditionType :type "/Game/ThirdPerson/Progression/E_ConditionType Enum" :default "NewEnumerator0") (ConditionTarget :type Name) (Amount :type Integer))
  (bind _returnvalue (`KismetStringLibrary.Conv_StringToName` (`KismetStringLibrary.Concat_StrStr` (`|GetEnumeratorNameAsString` ConditionType) ":" (`KismetStringLibrary.Conv_NameToString` ConditionTarget))))
  (bind _value (`self.GetCounter` _returnvalue))
  (`BlueprintMapLibrary.Map_Add` (`self.ProgressionCounters`) _returnvalue)
  (`self.EvaluateSteps`))